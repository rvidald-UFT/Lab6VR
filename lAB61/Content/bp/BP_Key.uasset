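; BP_Key is a key actor that opens a door when the third-person character overlaps it, provided the key carries the "key" tag.
; On BeginPlay, a tagged key applies its key material and stores the first BP_Puerta found in the level.
; On overlap, a Timeline lerps that door along Y between hardcoded relative positions, while the key itself stays in place.
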(event `self.ReceiveBeginPlay`
  (if (`self.ActorHasTag` "key")
    (`PrimitiveComponent.SetMaterial` (`self.kety`) 0 "/Game/mats/Mat_Llave.Mat_Llave")
    (bind _outactors (`GameplayStatics.GetAllActorsOfClass` "/Game/bp/BP_Puerta.BP_Puerta_C"))
    (set `self.Ref_puerta` (`|GetArrayItem` _outactors))))

(event `self.ReceiveActorBeginOverlap`
  (params (OtherActor :type "Actor Object Reference"))
  (cast `/Game/ThirdPerson/Blueprints/BP_ThirdPersonCharacter` OtherActor)
  (if (`self.ActorHasTag` "key")
    (bind (_direction _newtrack_0) (`Timeline|Timeline`)
      (:`Update`
        (`self.K2_SetActorRelativeLocation` (`self.Ref_puerta`) (`KismetMathLibrary.MakeVector` 1420.0 (`KismetMathLibrary.Lerp` -510.0 -170.0 _newtrack_0) 160.0) false false)))))

(fn `UserConstructionScript`)